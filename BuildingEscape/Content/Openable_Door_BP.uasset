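; Openable door actor that swings open and closed in response to its OpenDoor open and close request events.
; The Door_Swing timeline adds a yaw angle to the rotation captured at BeginPlay, playing forward to open and reversing to close.
; An event track on the timeline plays the Doorlock sound at InitialLocation, though the node that would set that location is never executed.
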(event OnOpenRequest(OpenDoor)
  (bind _open_angle (Timeline|Door_Swing Play)
    (:Update
      (Transformation|SetActorRotation (Math|Rotator|CombineRotators (stale EventBeginPlay _output_get) (Math|Rotator|MakeRotator 0.0 0.0 _open_angle))))
    (:NewTrack_1
      (Audio|PlaySoundatLocation "/Game/Audio/door-lock.door-lock" (stale _output_get) "0, 0, 0" 1.0 1.0 0.0 0 0 0))))

(event OnCloseRequest(OpenDoor)
  (bind _open_angle (Timeline|Door_Swing Reverse)
    (:Update
      (Transformation|SetActorRotation (Math|Rotator|CombineRotators (stale EventBeginPlay _output_get) (Math|Rotator|MakeRotator 0.0 0.0 _open_angle))))
    (:NewTrack_1
      (Audio|PlaySoundatLocation "/Game/Audio/door-lock.door-lock" (stale _output_get) "0, 0, 0" 1.0 1.0 0.0 0 0 0))))

(event EventBeginPlay
  (bind _output_get (Variables|Default|SetInitial_Rotation (Transformation|GetActorRotation))))

(fn ConstructionScript)